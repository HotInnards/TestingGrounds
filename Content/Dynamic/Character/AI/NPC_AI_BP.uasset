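; AI controller for guard NPCs that runs the GuardBehaviour behavior tree on the PatrolData blackboard from BeginPlay.
; Perception updates store any sensed actor not tagged "Enemy" in the blackboard's enemy key and clear the key when such an actor's stimulus is lost.
; Logic to set the pawn's aiming and shooting flags from the focus actor is present but disconnected from Tick, so it never runs.
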(event OnTargetPerceptionUpdated(AIPerception)
  (params (Actor :type Actor%20Object%20Reference) (Stimulus :type AI%20Stimulus%20Structure))
  ;[1 1 1] If the player is sensed, set blackboard values
  (CallFunction|UpdateBlackboardEnemyKey Actor Stimulus Actor))

(event EventBeginPlay
  ;[1 1 1] Set AI behaviour tree
  (bind _blackboardcomponent (Class|AIController|UseBlackboard "/Game/Dynamic/Character/AI/PatrolData.PatrolData"))
  (AI|RunBehaviorTree "/Game/Dynamic/Character/AI/GuardBehaviour.GuardBehaviour")
  (Variables|Default|SetBlackboardComponent _blackboardcomponent))

(event EventTick
  (params (DeltaSeconds :type Float%20%28single-precision%29))
  ;[1 1 1] Set aiming and shooting variables
)

(fn ConstructionScript)

(fn UpdateBlackboardEnemyKey
  (params (ObjectValue :type Object%20Object%20Reference) (AIStimulus :type AI%20Stimulus%20Structure%20%28by%20ref%29) (self2 :type Actor%20Object%20Reference))
  (bind _enemykey (Variables|Default|GetEnemyKey))
  (bind _blackboardcomponent (Variables|Default|GetBlackboardComponent))
  (if (not (Actor|ActorHasTag self2 "Enemy"))
    (if (.bSuccessfullySensed (Utilities|Struct|BreakAIStimulus AIStimulus))
      (AI|Components|Blackboard|SetValueasObject _blackboardcomponent _enemykey ObjectValue)
      (else
        (AI|Components|Blackboard|ClearValue _blackboardcomponent _enemykey)))))